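; Actor Blueprint that places instanced static meshes along a spline and spins each one around the spline's direction.
; On BeginPlay it adds instances at equal distances from start to end of the spline and caches their world transforms in an array.
; Tick combines a time-driven roll with each cached rotation and updates the instance, keeping its location and scale, so the spin stays local to the spline tangent.
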(event `self.ReceiveBeginPlay`
  (bind _spline (`self.Spline`))
  (for _index (range 9)
    (bind _returnvalue (`SplineComponent.GetTransformAtDistanceAlongSpline` _spline (* _index (/ (`SplineComponent.GetSplineLength` _spline) 8.0)) "World" false))
    (`InstancedStaticMeshComponent.AddInstance` (`self.InstancedStaticMesh`) _returnvalue true)
    (`KismetArrayLibrary.Array_Add` (`self.NewVar_0`) _returnvalue)))

(event `self.ReceiveTick`
  (params (DeltaSeconds :type "Float (single-precision)"))
  (bind _instancedstaticmesh (`self.InstancedStaticMesh`))
  (for (_array_element _array_index) (`self.NewVar_0`)
    (bind _outinstancetransform (`InstancedStaticMeshComponent.GetInstanceTransform` _instancedstaticmesh _array_index true))
    (`InstancedStaticMeshComponent.UpdateInstanceTransform` _instancedstaticmesh _array_index (`KismetMathLibrary.MakeTransform` (.location _outinstancetransform) (`KismetMathLibrary.ComposeRotators` (`KismetMathLibrary.MakeRotator` (* (`GameplayStatics.GetTimeSeconds`) 180.0)) (.rotation _array_element)) (.scale _outinstancetransform)) true true true)))

(fn `UserConstructionScript`)