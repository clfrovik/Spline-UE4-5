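; Spline Blueprint that lines a path with frame meshes and runs a looping glow and visibility sequence along them.
; The construction script adds spline mesh components at fixed Distance intervals, cycling through a mesh list.
; Offset looping timers advance separate on and off indices, with optional cycle limiting.
; After a start delay, Tick shows and hides the indexed frames, creating dynamic material instances each update to set color and luminosity.
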(event `Start`
  ;[1 1 1] Событие старта
  (set `self.By event or not` false))

(event `self.ReceiveBeginPlay`
  ;[1 1 1] Рассчёт всех индексов, изменение таймингов, времени
  ;;[0 1 0.08272] Включение рамок
  (`KismetSystemLibrary.K2_SetTimerDelegate` (delegate `EventVkl`) (`self.Appearance delay time`) true)
  ;;[1 0.8167 0] Расстояние между рамками зависит от этой паузы
  (`KismetSystemLibrary.Delay` (`self.Number of frame`))
  ;;[1 0.06951 0] Отключение рамок
  (`KismetSystemLibrary.K2_SetTimerDelegate` (delegate `Event Vikl`) (`self.Shutdown delay time`) true))

(event `EventVkl`
  ;[1 1 1] Рассчёт всех индексов, изменение таймингов, времени
  (if (`self.Infinity of the cycle`)
    (bind _output_get (set `self.Index Vkl` (+ (`self.Index Vkl`) 1) :!label _label))
    (if (>= _output_get (`KismetArrayLibrary.Array_Length` (`self.Mesh`)))
      (set `self.Index Vkl` 0))
    (elif (not (== (`self.Cycl num N`) (`self.Cycl N`)))
      (goto _label))))

(event `Event Vikl`
  (bind _index_vikl (`self.Index vikl`))
  ;[1 1 1] Рассчёт всех индексов, изменение таймингов, времени
  (set `self.Index vikl` (+ _index_vikl 1))
  (if (>= _index_vikl (`KismetArrayLibrary.Array_Length` (`self.Mesh`)))
    (set `self.Index vikl` 0)
    ;;[0 0.3114 1] Просчёт
    (if (>= (`self.Index`) (`KismetArrayLibrary.Array_Length` (`self.Mesh`)))
      (set `self.Cycl N` (+ (`self.Cycl N`) 1)))))

(event `self.ReceiveTick`
  (params (DeltaSeconds :type "Float (single-precision)"))
  (bind _output (`|GetArrayItem` (`self.Mesh`) (`self.Index vikl`)))
  (bind _output_2 (`|GetArrayItem` (`self.Mesh`) (`self.Index Vkl`)))
  ;[1 0.6384 0.9307] Включение и отключение рамок, настройки
  (if (`self.Delay Check`)
    (`|ExecutionSequence`
      (:`then_1`
        (if (not (`self.By event or not`))
          (`SceneComponent.SetVisibility` _output_2 true false)
          (bind _returnvalue (`PrimitiveComponent.CreateDynamicMaterialInstance` _output_2 0 "/Game/Blueprints/Cube_m.Cube_m" "None"))
          (`MaterialInstanceDynamic.SetVectorParameterValue` _returnvalue "Param1" (`self.Color`))
          (`MaterialInstanceDynamic.SetScalarParameterValue` _returnvalue "Param" (`self.Luminosity`))
          (`SceneComponent.SetVisibility` _output false false)
          (bind _returnvalue_2 (`PrimitiveComponent.CreateDynamicMaterialInstance` _output 0 "/Game/Blueprints/Cube_m.Cube_m" "None"))
          (`MaterialInstanceDynamic.SetScalarParameterValue` _returnvalue_2 "Param" (`self.luminosity zero`)))))
    (else
      (`KismetSystemLibrary.Delay` (`self.Start Delay`))
      (set `self.Delay Check` true))))

(fn `UserConstructionScript`
  (bind _spline (`self.Spline`))
  (bind _index_of_frame (`self.Index of Frame`))
  (bind _spline_2 (`self.Spline`))
  ;[1 1 1] Создание рамок по сплайну
  (for _index (range (+ (`KismetMathLibrary.FTrunc` (/ (`SplineComponent.GetSplineLength` (`self.Spline`)) (`self.Distance`))) 1))
    (if (not (`self.1`))
      (bind _returnvalue (`AddComponent|NODE_AddSplineMeshComponent-0`))
      (`StaticMeshComponent.SetStaticMesh` _returnvalue (`|GetArrayItem` (`self.meshh`) (`self.Index of Frame`)))
      (`SceneComponent.SetVisibility` _returnvalue true false)
      (set `self.Spline Mesh Component` _returnvalue)
      (`KismetArrayLibrary.Array_Set` (`self.Mesh`) (`self.index`) _returnvalue true)
      (set `self.Index of Frame` (+ _index_of_frame 1))
      (if (>= _index_of_frame (`KismetArrayLibrary.Array_Length` (`self.meshh`)))
        (set `self.Index of Frame` 0))
      (set `self.Angle(bp)` (+ (`self.Angle(bp)`) (`self.Angle`)))
      (set `self.index` (+ (`self.index`) 1))
      (`SplineMeshComponent.SetForwardAxis` (`self.Spline Mesh Component`) "X" true)
      (bind _returnvalue_2 (* _index (`self.Distance`)))
      (bind _returnvalue_3 (* (+ _index 0) (`self.Distance`)))
      (`SplineMeshComponent.SetStartAndEnd` (`self.Spline Mesh Component`) (`SplineComponent.GetLocationAtDistanceAlongSpline` _spline_2 _returnvalue_2 "Local") (`KismetMathLibrary.ClampVectorSize` (`SplineComponent.GetTangentAtDistanceAlongSpline` _spline_2 _returnvalue_2 "Local") 0.0 (`self.Distance`)) (`SplineComponent.GetLocationAtDistanceAlongSpline` _spline _returnvalue_3 "Local") (`KismetMathLibrary.ClampVectorSize` (`SplineComponent.GetTangentAtDistanceAlongSpline` _spline _returnvalue_3 "Local") 0.0 (`self.Distance`)) true)
      (`PrimitiveComponent.SetCollisionEnabled` (`self.Spline Mesh Component`) "QueryAndPhysics"))))